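; Helper functions for master server communication, covering HTTP request structs and server information structs.
; Setters rebuild the request struct with a new data or destination value, copying the other fields.
; The request-type setter maps register, unregister and check-in to a JSON field with PUT, and server-list retrieval to a query destination, without storing the passed type.
; An address getter joins a server's IP and port.
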(fn FHttpRequest-SetData
  (params (HttpRequest :type Http%20Request%20Structure) (NewData :type String))
  (bind (_thedest _thedata _mid _qid _delim _requestverb _requesttype _jsonobjectfield _responsetype) (Utilities|Struct|BreakHttpRequest HttpRequest))
  (Utilities|Struct|SetmembersinHttpRequest (Utilities|Struct|MakeHttpRequest _thedest NewData _mid _qid _delim _requestverb _requesttype _jsonobjectfield _responsetype)))

(fn FHttpRequest-SetDestination
  (params (HttpRequest :type Http%20Request%20Structure) (NewDestination :type String))
  (bind (_thedest _thedata _mid _qid _delim _requestverb _requesttype _jsonobjectfield _responsetype) (Utilities|Struct|BreakHttpRequest HttpRequest))
  (Utilities|Struct|SetmembersinHttpRequest (Utilities|Struct|MakeHttpRequest NewDestination _thedata _mid _qid _delim _requestverb _requesttype _jsonobjectfield _responsetype)))

(fn FHttpRequest-SetRequestType
  (params (HttpRequest :type Http%20Request%20Structure) (RequestType :type EHttpRequestType%20Enum))
  (bind (_thedest _thedata _mid _qid _delim _requestverb _requesttype _jsonobjectfield _responsetype) (Utilities|Struct|BreakHttpRequest HttpRequest))
  (bind (_thedest_2 _thedata_2 _mid_2 _qid_2 _delim_2 _requestverb_2 _requesttype_2 _jsonobjectfield_2 _responsetype_2) (Utilities|Struct|BreakHttpRequest HttpRequest))
  (switch Utilities|FlowControl|Switch|SwitchonEHttpRequestType RequestType
    (:HRT_RegisterServer
      (LocalVariables|SetJsonObjectField "ServerRegistration")
      (LocalVariables|SetVerb "PUT" :!label _label)
      (Utilities|Struct|SetmembersinHttpRequest (Utilities|Struct|MakeHttpRequest _thedest_2 _thedata_2 _mid_2 _qid_2 _delim_2 (LocalVariables|GetVerb) _requesttype_2 (LocalVariables|GetJsonObjectField) _responsetype_2)))
    (:HRT_UnregisterServer
      (LocalVariables|SetJsonObjectField "ServerDeregistration")
      (goto _label))
    (:HRT_CheckIn
      (LocalVariables|SetJsonObjectField "ServerCheckIn")
      (goto _label))
    (:HRT_ReceiveServerList
      (Utilities|Struct|SetmembersinHttpRequest (Utilities|Struct|MakeHttpRequest "/?ReceiveServerList=True" _thedata _mid _qid _delim "GET" _requesttype _jsonobjectfield _responsetype)))))

(fn FServerInformation-GetFullAddress
  (params (ServerInformation :type Server%20Information%20Structure))
  (bind (_name _ip _port) (Utilities|Struct|BreakServerInformation ServerInformation))
  (return (Utilities|String|Append _ip ":" _port)))